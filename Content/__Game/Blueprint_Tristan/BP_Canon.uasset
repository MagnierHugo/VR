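; BP_Canon is a cannon actor that fires projectiles in the direction of the ball.
; On BeginPlay it caches the BP_Ball actor and starts a looping one-second timer that calls Shoot by name.
; Shoot snaps the whole actor to face the ball's current position through LookAt, then spawns a BP_Projectile at the actor's location and rotation.
; Aim updates only at each shot, with no continuous tracking or target leading.
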(event `self.ReceiveBeginPlay`
  (bind _returnvalue (`GameplayStatics.GetActorOfClass` "/Game/__Game/Blueprint_Tristan/BP_Ball.BP_Ball_C"))
  (set `self.Ball` _returnvalue)
  (`KismetSystemLibrary.K2_SetTimer` null "Shoot" 1.0 true true))

(fn `LookAt`
  (`self.K2_SetActorRotation` (`KismetMathLibrary.FindLookAtRotation` (`SceneComponent.K2_GetComponentLocation`) (`SceneComponent.K2_GetComponentLocation` (`Actor.RootComponent` (`self.Ball`))))))

(fn `Shoot`
  (`self.LookAt`)
  (`|SpawnActorFromClass` "/Game/__Game/Blueprint_Tristan/BP_Projectile.BP_Projectile_C" (`KismetMathLibrary.MakeTransform` (`self.K2_GetActorLocation`) (`self.K2_GetActorRotation`)) "AlwaysSpawn" "MultiplyWithRoot" null null))

(fn `UserConstructionScript`)
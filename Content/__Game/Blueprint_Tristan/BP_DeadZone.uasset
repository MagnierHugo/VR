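; BP_DeadZone is a lose-condition trigger that reacts when a BP_Ball overlaps its box.
; On BeginPlay it caches the referenced platform's transform, plus the player controller's transform, which goes unused.
; On overlap it waits, prints a "Looser" message, waits again, then destroys the platform and spawns a fresh BP_Plat at the cached transform.
; The platform reference is not reassigned to the newly spawned actor.
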(event `self.ReceiveBeginPlay`
  ; Setup Variable
  (set `self.PlayerPos` (`self.GetTransform` (`GameplayStatics.GetPlayerController` 0)))
  (set `self.PlatPos` (`self.GetTransform` (`self.BP Plat`))))

(event `self.Box.OnComponentBeginOverlap`
  (params (OverlappedComponent :type "PrimitiveComponent Object Reference") (OtherActor :type "Actor Object Reference") (OtherComp :type "PrimitiveComponent Object Reference") (OtherBodyIndex :type Integer) (bFromSweep :type Boolean) (SweepResult :type "HitResult Structure (by ref)"))
  ; Loose Condition
  (cast `/Game/__Game/Blueprint_Tristan/BP_Ball` OtherActor)
  (`KismetSystemLibrary.Delay` 2.0)
  (`KismetSystemLibrary.PrintString` "Looser" true true (struct :`R` 0.484375 :`B` 0.027763 :`A` 1.0) 15.0 "tj")
  (`KismetSystemLibrary.Delay` 2.0)
  (`self.K2_DestroyActor` (`self.BP Plat`))
  (`|SpawnActorFromClass` "/Game/__Game/Blueprint_Tristan/BP_Plat.BP_Plat_C" (`self.PlatPos`) "Undefined" "MultiplyWithRoot" null null))

(fn `UserConstructionScript`)
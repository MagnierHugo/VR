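; Level manager for the Beat Saber minigame that spawns BP_Cube actors for a limited duration.
; BeginPlay caches the BP_DeleteMissedCube actor and sets a short timer that calls SpawnCube, repeating according to the Looping variable.
; While StartLevel is true and Tick-accumulated time is within DurationGame, cubes spawn at random width and height offsets from the manager.
; Past that duration it clears Looping, without clearing the timer itself.
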(event `self.ReceiveTick`
  (params (DeltaSeconds :type "Float (single-precision)"))
  ; clock
  (set `self.TimeElapsed` (+ DeltaSeconds (`self.TimeElapsed`))))

(event `self.ReceiveBeginPlay`
  ; loop for projspawn
  (bind _returnvalue (`GameplayStatics.GetActorOfClass` "/Game/__Game/Blueprints/BeatSaber/BP/BP_DeleteMissedCube.BP_DeleteMissedCube_C"))
  (set `self.EnterLevel` _returnvalue)
  (`KismetSystemLibrary.K2_SetTimerDelegate` (delegate `SpawnCube`) 0.3 (`self.Looping`)))

(event `SpawnCube`
  ; SpawnCube Behavior
  (if (`self.startLevel`)
    (if (<= (`self.TimeElapsed`) (`self.DurationGame`))
      (`|SpawnActorFromClass` "/Game/__Game/Blueprints/BeatSaber/BP/BP_Cube.BP_Cube_C" (`KismetMathLibrary.MakeTransform` (+ (`self.K2_GetActorLocation`) (`KismetMathLibrary.MakeVector` (`KismetMathLibrary.RandomFloatInRange` 0.0 (`self.MaxSpawnWidht`)) 0.0 (`KismetMathLibrary.RandomFloatInRange` (`self.MinSpawnHeight`)))) (struct :`Yaw` -90.0)) "AdjustIfPossibleButAlwaysSpawn" "MultiplyWithRoot" null null)
      (else
        (set `self.Looping` false)))))

(fn `UserConstructionScript`)
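; BP_Sabre is a grabbable, colored saber for a Beat Saber-style game, with its material set by IsBlue at BeginPlay.
; Grabbing it sets StartLevel on BP_BeatSaberLevelManager.
; Overlapping a BP_Cube of matching color spawns impact Niagara, plays haptics on the color's hand (blue is right), increments the manager's score and destroys the cube.
; Each hit ends with a brief global time dilation for hit-stop.
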(event `self.ReceiveBeginPlay`
  ; Apply Color & get levelmanager reference
  (if (`self.isBlue`)
    (`PrimitiveComponent.SetMaterial` (`self.Cube1`) 0 "/Engine/TemplateResources/MI_Template_BaseBlue.MI_Template_BaseBlue")
    (`PrimitiveComponent.SetMaterial` (`self.Cube`) 0 "/Engine/TemplateResources/MI_Template_BaseBlue.MI_Template_BaseBlue")
    (else
      (`PrimitiveComponent.SetMaterial` (`self.Cube1`) 0 "/Engine/EngineDebugMaterials/MAT_LevelColorationLitLightmapUV.MAT_LevelColorationLitLightmapUV")
      (`PrimitiveComponent.SetMaterial` (`self.Cube`) 0 "/Engine/EngineDebugMaterials/MAT_LevelColorationLitLightmapUV.MAT_LevelColorationLitLightmapUV")))
  (bind _returnvalue (`GameplayStatics.GetActorOfClass` "/Game/__Game/Blueprints/BeatSaber/BP/BP_BeatSaberLevelManager.BP_BeatSaberLevelManager_C")))

(event `self.Collision.OnComponentBeginOverlap`
  (params (OverlappedComponent :type "PrimitiveComponent Object Reference") (OtherActor :type "Actor Object Reference") (OtherComp :type "PrimitiveComponent Object Reference") (OtherBodyIndex :type Integer) (bFromSweep :type Boolean) (SweepResult :type "HitResult Structure (by ref)"))
  (bind _returnvalue (`GameplayStatics.GetPlayerController` 0))
  ; Collision with cube behavior, check right left, play haptic and hit impact with score
  (bind _asbp_cube (cast `/Game/__Game/Blueprints/BeatSaber/BP/BP_Cube` OtherActor))
  (if (== (`/Game/__Game/Blueprints/BeatSaber/BP/BP_Cube.isBlue` _asbp_cube) (`self.isBlue`))
    (`NiagaraFunctionLibrary.SpawnSystemAtLocation` "/Game/__Game/Blueprints/BeatSaber/FX/NS_CubeImpact.NS_CubeImpact" (`self.K2_GetActorLocation` _asbp_cube))
    (if (`self.isBlue`)
      (`PlayerController.PlayHapticEffect` _returnvalue "/Game/__Game/Blueprints/BeatSaber/FX/Haptic_CubeHit.Haptic_CubeHit" "Right" 1.0 false)
      (else
        (`PlayerController.PlayHapticEffect` _returnvalue "/Game/__Game/Blueprints/BeatSaber/FX/Haptic_CubeHit.Haptic_CubeHit" "Left" 1.0 false)))
    (set `/Game/__Game/Blueprints/BeatSaber/BP/BP_BeatSaberLevelManager.PlayerScore` (+ (`/Game/__Game/Blueprints/BeatSaber/BP/BP_BeatSaberLevelManager.PlayerScore` (stale `self.ReceiveBeginPlay` _returnvalue)) 1) (stale `self.ReceiveBeginPlay` _returnvalue))
    (`self.K2_DestroyActor` _asbp_cube)
    (`GameplayStatics.SetGlobalTimeDilation` 0.05)
    (`KismetSystemLibrary.Delay` 0.03)
    (`GameplayStatics.SetGlobalTimeDilation` 1.0)))

(event `self.GrabComponent.OnGrabbed`
  ; Start game on grab
  (set `/Game/__Game/Blueprints/BeatSaber/BP/BP_BeatSaberLevelManager.startLevel` true (stale `self.ReceiveBeginPlay` _returnvalue)))

(fn `UserConstructionScript`)
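; Level spawner actor for a Beat Saber-style game that spawns BP_Cube actors during a timed round.
; A timer set at BeginPlay calls SpawnCube, which places each cube at a random X offset from the actor with a fixed rotation.
; Tick accumulates elapsed time; past DurationGame, spawning stops and Looping is set false, though the timer itself is never cleared.
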(event `self.ReceiveTick`
  (params (DeltaSeconds :type "Float (single-precision)"))
  (set `self.TimeElapsed` (+ DeltaSeconds (`self.TimeElapsed`))))

(event `self.ReceiveBeginPlay`
  (`KismetSystemLibrary.K2_SetTimerDelegate` (delegate `SpawnCube`) 0.4 (`self.Looping`)))

(event `SpawnCube`
  (if (<= (`self.TimeElapsed`) (`self.DurationGame`))
    (`|SpawnActorFromClass` "/Game/__Game/Blueprints/BeatSaber/BP_Cube.BP_Cube_C" (`KismetMathLibrary.MakeTransform` (+ (`self.K2_GetActorLocation`) (`KismetMathLibrary.MakeVector` (`KismetMathLibrary.RandomFloatInRange` 0.0 (`self.MaxSpawnWidht`)))) (struct :`Yaw` -90.0)) "AdjustIfPossibleButAlwaysSpawn" "MultiplyWithRoot" null null)
    (else
      (set `self.Looping` false))))

(fn `UserConstructionScript`)
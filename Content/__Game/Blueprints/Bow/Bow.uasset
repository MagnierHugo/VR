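; VR bow actor that the player holds in one hand and draws with the other to fire arrows.
; Grabbing the string grip starts a looping timer that sets pull strength from the free hand's distance to it; only the left-hand path divides by max pull length.
; AttachArrow swaps an arrow actor for the built-in mesh; releasing the grip hides it and spawns an ArrowShoot at that speed.
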(event `self.ReceiveBeginPlay`
  ; Get the player's VRPawn
  (bind _asvrpawn (cast `/Game/VRTemplate/Blueprints/VRPawn` (`GameplayStatics.GetPlayerPawn` 0)))
  (set `self.Player` _asvrpawn))

(event `self.GrabComponent.OnGrabbed`
  ; Which hand is holding the bow
  (set `self.RightHeld` (== (`/Game/VRTemplate/Blueprints/VRPawn.HeldComponentRight` (`self.Player`)) (`self.GrabComponent`))))

(event `self.GrabComponent1.OnGrabbed`
  ; Calculate pulling force following the pulling hand
  (`KismetSystemLibrary.K2_SetTimerDelegate` (delegate `PullBow`) 0.2 true))

(event `PullBow`
  ; Calculate pulling force following the pulling hand
  (if (`self.RightHeld`)
    (`self.LeftHandPull`)
    (else
      (`self.RightHandPull`))))

(event `self.GrabComponent1.OnDropped`
  ; Shoot the arrow
  (if (`self.Has Arrow`)
    (`self.ShootArrow` (`self.Pull Strength`) (`KismetMathLibrary.MakeTransform` (`SceneComponent.K2_GetComponentLocation` (`self.cc0_wooden_arrow`)) (`self.K2_GetActorRotation`)))
    (set `self.Has Arrow` false)
    (`SceneComponent.SetVisibility` (`self.cc0_wooden_arrow`) false false)))

(fn `AttachArrow`
  (params (Arrow :type "/Game/__Game/Blueprints/Arrow/Arrow Object Reference"))
  (`self.K2_DestroyActor` Arrow)
  (`SceneComponent.SetVisibility` (`self.cc0_wooden_arrow`) true false)
  (set `self.Has Arrow` true))

(fn `LeftHandPull`
  (set `self.Pull Strength` (`KismetMathLibrary.Lerp` 0.0 (`self.Max Pull Strengh`) (/ (`KismetMathLibrary.VSize` (- (`SceneComponent.K2_GetComponentLocation` (`/Game/VRTemplate/Blueprints/VRPawn.MotionControllerLeftGrip` (`self.Player`))) (`SceneComponent.K2_GetComponentLocation` (`self.GrabComponent1`)))) (`self.Max Pull Length`)))))

(fn `RightHandPull`
  (set `self.Pull Strength` (`KismetMathLibrary.Lerp` 0.0 (`self.Max Pull Strengh`) (`KismetMathLibrary.VSize` (- (`SceneComponent.K2_GetComponentLocation` (`/Game/VRTemplate/Blueprints/VRPawn.MotionControllerRightGrip` (`self.Player`))) (`SceneComponent.K2_GetComponentLocation` (`self.GrabComponent1`)))))))

(fn `ShootArrow`
  (params (`Initial Speed` :type "Float (single-precision)") (SpawnTransform :type "Transform Structure"))
  (`|SpawnActorFromClass` "/Game/__Game/Blueprints/Arrow/ArrowShoot.ArrowShoot_C" SpawnTransform "AlwaysSpawn" "MultiplyWithRoot" null `Initial Speed` null)
  (`KismetSystemLibrary.PrintString` (`KismetStringLibrary.Conv_DoubleToString` `Initial Speed`) true true (struct :`G` 0.66 :`B` 1.0 :`A` 1.0) 10.0 "arrow:throw"))

(fn `UserConstructionScript`)
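; VR two-handed sniper rifle that attaches its scope capture and magazine at BeginPlay and constrains its lever by physics.
; Grabbing either grip hides hand messages and adds a hand-specific weapon input context, both keyed to the secondary grip's hand.
; That hand's shoot input fires only with both grips held and a chambered bullet.
; Firing is currently just a short debug-drawn line trace from the nozzle, with no hit handling.
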(event `self.ReceiveBeginPlay`
  (bind _sniper (`self.Sniper`))
  ; Begin
  (`SceneComponent.K2_AttachToComponent` (`self.Lunette de rendu`) _sniper "None" "KeepRelative" "KeepRelative" "KeepRelative" true)
  (`SceneComponent.K2_AttachToComponent` (`self.SceneCaptureComponent2D`) _sniper "None" "KeepRelative" "KeepRelative" "KeepRelative" true)
  (`SceneComponent.K2_AttachToComponent` (`self.Magazine`) _sniper "None" "KeepRelative" "KeepRelative" "KeepRelative" true)
  (`PhysicsConstraintComponent.SetConstrainedComponents` (`self.PhysicsConstraint`) _sniper "None" (`self.Sniper_lever_V4`) "None"))

(event `self.GrabComponentMain.OnGrabbed`
  (bind _grabcomponentsecondary (`self.GrabComponentSecondary`))
  (bind _returnvalue (`|EnumEquality` (`/Game/VRTemplate/Blueprints/GrabComponent.GetHeldByHand` _grabcomponentsecondary) "Right"))
  ; Grab Main
  (`self.EnableInput` (`GameplayStatics.GetPlayerController` 0))
  (message `/Game/VRTemplate/Blueprints/BPI_PawnAnim.HideUnhideHand` (`ActorComponent.GetOwner` (`/Game/VRTemplate/Blueprints/GrabComponent.MotionControllerRef` _grabcomponentsecondary)) true _returnvalue)
  (`EnhancedInputSubsystemInterface.AddMappingContext` (pcsubsystem `EnhancedInputLocalPlayerSubsystem` (`GameplayStatics.GetPlayerController` 0)) (select `bool` _returnvalue :`false` "/Game/VRTemplate/Input/IMC_Weapon_Left.IMC_Weapon_Left" :`true` "/Game/VRTemplate/Input/IMC_Weapon_Right.IMC_Weapon_Right" :!type "InputMappingContext Object Reference") 1 (struct))
  (set `self.MainIsGrab?` true))

(event `self.GrabComponentMain.OnDropped`
  (bind _grabcomponentsecondary (`self.GrabComponentSecondary`))
  (bind _returnvalue (`|EnumEquality` (`/Game/VRTemplate/Blueprints/GrabComponent.GetHeldByHand` _grabcomponentsecondary) "Right"))
  ; Grab Main
  (`self.DisableInput` (`GameplayStatics.GetPlayerController` 0))
  (message `/Game/VRTemplate/Blueprints/BPI_PawnAnim.HideUnhideHand` (`ActorComponent.GetOwner` (`/Game/VRTemplate/Blueprints/GrabComponent.MotionControllerRef` _grabcomponentsecondary)) false _returnvalue)
  (`EnhancedInputSubsystemInterface.RemoveMappingContext` (pcsubsystem `EnhancedInputLocalPlayerSubsystem` (`GameplayStatics.GetPlayerController` 0)) (select `bool` _returnvalue :`false` "/Game/VRTemplate/Input/IMC_Weapon_Left.IMC_Weapon_Left" :`true` "/Game/VRTemplate/Input/IMC_Weapon_Right.IMC_Weapon_Right" :!type "InputMappingContext Object Reference") (struct))
  (set `self.MainIsGrab?` false))

(event `self.GrabComponentSecondary.OnGrabbed`
  (bind _grabcomponentsecondary (`self.GrabComponentSecondary`))
  (bind _returnvalue (`|EnumEquality` (`/Game/VRTemplate/Blueprints/GrabComponent.GetHeldByHand` _grabcomponentsecondary) "Right"))
  ; Grab Secondary
  (`self.EnableInput` (`GameplayStatics.GetPlayerController` 0))
  (message `/Game/VRTemplate/Blueprints/BPI_PawnAnim.HideUnhideHand` (`ActorComponent.GetOwner` (`/Game/VRTemplate/Blueprints/GrabComponent.MotionControllerRef` _grabcomponentsecondary)) true _returnvalue)
  (`EnhancedInputSubsystemInterface.AddMappingContext` (pcsubsystem `EnhancedInputLocalPlayerSubsystem` (`GameplayStatics.GetPlayerController` 0)) (select `bool` _returnvalue :`false` "/Game/VRTemplate/Input/IMC_Weapon_Left.IMC_Weapon_Left" :`true` "/Game/VRTemplate/Input/IMC_Weapon_Right.IMC_Weapon_Right" :!type "InputMappingContext Object Reference") 1 (struct))
  (set `self.SecondaryIsGrab?` true))

(event `self.GrabComponentSecondary.OnDropped`
  (bind _grabcomponentsecondary (`self.GrabComponentSecondary`))
  (bind _returnvalue (`|EnumEquality` (`/Game/VRTemplate/Blueprints/GrabComponent.GetHeldByHand` _grabcomponentsecondary) "Right"))
  ; Grab Secondary
  (`self.DisableInput` (`GameplayStatics.GetPlayerController` 0))
  (message `/Game/VRTemplate/Blueprints/BPI_PawnAnim.HideUnhideHand` (`ActorComponent.GetOwner` (`/Game/VRTemplate/Blueprints/GrabComponent.MotionControllerRef` _grabcomponentsecondary)) false _returnvalue)
  (`EnhancedInputSubsystemInterface.RemoveMappingContext` (pcsubsystem `EnhancedInputLocalPlayerSubsystem` (`GameplayStatics.GetPlayerController` 0)) (select `bool` _returnvalue :`false` "/Game/VRTemplate/Input/IMC_Weapon_Left.IMC_Weapon_Left" :`true` "/Game/VRTemplate/Input/IMC_Weapon_Right.IMC_Weapon_Right" :!type "InputMappingContext Object Reference") (struct))
  (set `self.SecondaryIsGrab?` false))

(event `EnhancedInput|/Game/VRTemplate/Input/Actions/IA_Shoot_Left`
  (params (ActionValue :type Boolean) (ElapsedSeconds :type "Float (double-precision)") (TriggeredSeconds :type "Float (double-precision)") (InputAction :type "InputAction Object Reference" :default "/Game/VRTemplate/Input/Actions/IA_Shoot_Left.IA_Shoot_Left"))
  ; Shoot
  (:`Started`
    (if (`|EnumEquality` (`/Game/VRTemplate/Blueprints/GrabComponent.GetHeldByHand` (`self.GrabComponentSecondary`)) "Left")
      (`self.TryToShoot` :!label _label))))

(event `EnhancedInput|/Game/VRTemplate/Input/Actions/IA_Shoot_Right`
  (params (ActionValue :type Boolean) (ElapsedSeconds :type "Float (double-precision)") (TriggeredSeconds :type "Float (double-precision)") (InputAction :type "InputAction Object Reference" :default "/Game/VRTemplate/Input/Actions/IA_Shoot_Right.IA_Shoot_Right"))
  ; Shoot
  (:`Started`
    (if (`|EnumEquality` (`/Game/VRTemplate/Blueprints/GrabComponent.GetHeldByHand` (`self.GrabComponentSecondary`)) "Right")
      (goto _label))))

(event `TryToShoot`
  (bind _nozzle (`self.Nozzle`))
  (bind _returnvalue (`SceneComponent.K2_GetComponentLocation` _nozzle))
  ; Try To Shoot
  (if (and (`self.MainIsGrab?`) (`self.SecondaryIsGrab?`) (`self.Bullet_in_chamber`))
    (`KismetSystemLibrary.LineTraceSingle` :`Start` _returnvalue :`End` (+ _returnvalue (* (`SceneComponent.GetForwardVector` _nozzle) 500.0)) :`TraceChannel` "TraceTypeQuery1" :`DrawDebugType` "ForDuration")
    (else
      (`KismetSystemLibrary.PrintString` "Unauthorised shooting"))))

(fn `UserConstructionScript`)
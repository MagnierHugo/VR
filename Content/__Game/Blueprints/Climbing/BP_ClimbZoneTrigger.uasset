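; BP_ClimbZoneTrigger is a trigger actor that marks an area where the VR player is allowed to climb.
; When a VRPawn begins overlapping it, the trigger sets the pawn's CanClimb flag to true, and clears it when the overlap ends.
; Both transitions print a debug string, and leftover stamina-widget visibility nodes are disconnected and never run.
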(event `self.ReceiveActorBeginOverlap`
  (params (OtherActor :type "Actor Object Reference"))
  (bind _asvrpawn (cast `/Game/VRTemplate/Blueprints/VRPawn` OtherActor))
  (set `/Game/VRTemplate/Blueprints/VRPawn.CanClimb` true _asvrpawn)
  (`KismetSystemLibrary.PrintString` "can climb"))

(event `self.ReceiveActorEndOverlap`
  (params (OtherActor :type "Actor Object Reference"))
  (bind _asvrpawn (cast `/Game/VRTemplate/Blueprints/VRPawn` OtherActor))
  (set `/Game/VRTemplate/Blueprints/VRPawn.CanClimb` false _asvrpawn)
  (`KismetSystemLibrary.PrintString` "can't climb"))

(fn `UserConstructionScript`)
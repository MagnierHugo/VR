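; Cannon actor that repeatedly fires at the BP_Ball found in the level.
; A looping timer moves it each second to a random point on a half-sphere around the ball, built from chained vector rotations, then turns it toward the ball.
; It spawns a scaled-down actor from that transform and prints the running shot count.
; At the shot limit it calls WinCondition on Plat and pauses the timer.
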(event `self.ReceiveBeginPlay`
  (bind _returnvalue (`GameplayStatics.GetActorOfClass` "/Game/__Game/Blueprints/Serveur/BP_Ball.BP_Ball_C"))
  (set `self.Ball` _returnvalue)
  (`KismetSystemLibrary.K2_SetTimer` null "Shoot" 1.0 true true))

(fn `GetRandomPointOnHalfSphere`
  (params (ActorLoc :type "Vector Structure"))
  (returns (ReturnVect :type "Vector Structure"))
  (return (+ ActorLoc (`KismetMathLibrary.RotateAngleAxis` (`KismetMathLibrary.RotateAngleAxis` (`KismetMathLibrary.RotateAngleAxis` (`KismetMathLibrary.MakeVector` 250.0) (`KismetMathLibrary.RandomFloatInRange` 0.0 180.0) (0.0 0.0 1.0)) (`KismetMathLibrary.RandomFloatInRange` 0.0 180.0) (0.0 1.0 0.0)) 90.0 (1.0 0.0 0.0)))))

(fn `LookAtBall`
  (returns (NewRotator :type "Rotator Structure"))
  (return (`KismetMathLibrary.FindLookAtRotation` (`self.K2_GetActorLocation`) (`SceneComponent.K2_GetComponentLocation` (`Actor.RootComponent` (`self.Ball`))))))

(fn `SetLocRotCanon`
  (params (ActorLoc :type "Vector Structure"))
  (bind _returnvect (`self.GetRandomPointOnHalfSphere` ActorLoc))
  (`self.K2_SetActorLocation` _returnvect)
  (bind _newrotator (`self.LookAtBall`))
  (`self.K2_SetActorRotation` _newrotator)
  (return))

(fn `Shoot`
  (`self.SetLocRotCanon` (`self.K2_GetActorLocation` (`self.Ball`)))
  (`|SpawnActorFromClass` "/Game/__Game/Blueprints/Serveur/BP_Projectile.BP_Projectile_C" (`KismetMathLibrary.MakeTransform` (`self.K2_GetActorLocation`) (`self.K2_GetActorRotation`) (0.25 0.25 0.25)) "AlwaysSpawn" "MultiplyWithRoot" null null)
  (bind _output_get (set `self.BallShoot` (+ (`self.BallShoot`) 1)))
  (`KismetSystemLibrary.PrintString` (`KismetStringLibrary.Conv_IntToString` _output_get))
  (if (== _output_get 60)
    (`/Game/__Game/Blueprints/Serveur/BP_Plat.WinCondition` (`self.Plat`))
    (`KismetSystemLibrary.K2_PauseTimer` null "Shoot")))

(fn `UserConstructionScript`)
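; BP_Plat is a grabbable VR plate carrying a ball, in what appears to be a waiter ("Serveur") minigame.
; Grabbing it spawns a BP_Canon at a random point around the ball, using chained vector rotations meant to pick from a half-sphere.
; Tick plays a left-hand haptic pulse while the ball's speed exceeds a warning threshold.
; A WinCondition event checks that the ball is valid, then calls Win, which only prints a message.
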(event `self.ReceiveBeginPlay`
  ; Launch Game
)

(event `self.GrabComponent.OnGrabbed`
  ; Launch Game
  (bind _returnvalue (`self.GetRandomPointOnHalfSphere` (`SceneComponent.K2_GetComponentLocation` (`self.BP_Ball`))))
  (bind _returnvalue_2 (`|SpawnActorFromClass` "/Game/__Game/Blueprints/Serveur/BP_Canon.BP_Canon_C" (`KismetMathLibrary.MakeTransform` _returnvalue) "AlwaysSpawn" "MultiplyWithRoot" null null))
  (set `self.Canon` _returnvalue_2))

(event `WinCondition`
  ; Win Condition
  (if (`KismetSystemLibrary.IsValid` (`self.BP_Ball`))
    (`self.Win`)))

(event `Win`
  ; Win Action
  (`KismetSystemLibrary.PrintString` "Win Ballon become"))

(event `self.ReceiveTick`
  (params (DeltaSeconds :type "Float (single-precision)"))
  (if (> (`KismetMathLibrary.VSize` (`SceneComponent.GetComponentVelocity` (`self.BP_Ball`))) (`self.minVelocityToWarnAboutRoll`))
    (`PlayerController.PlayHapticEffect` (`GameplayStatics.GetPlayerController` 0) "/Game/VRTemplate/Haptics/PistolFireHapticEffect.PistolFireHapticEffect" "Left" 1.0 false)))

(fn `GetRandomPointOnHalfSphere`
  (params (SphereLocation :type "Vector Structure"))
  (returns (ReturnValue :type "Vector Structure"))
  (return (+ (`KismetMathLibrary.RotateAngleAxis` (`KismetMathLibrary.RotateAngleAxis` (`KismetMathLibrary.RotateAngleAxis` (`KismetMathLibrary.MakeVector` 250.0) (`KismetMathLibrary.RandomFloatInRange` 0.0 180.0) (0.0 0.0 1.0)) (`KismetMathLibrary.RandomFloatInRange` 0.0 180.0) (0.0 1.0 0.0)) 90.0 (1.0 0.0 0.0)) SphereLocation)))

(fn `UserConstructionScript`)
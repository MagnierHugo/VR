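; Sniper empty bullet actor that removes itself from the world once its lifetime runs out.
; Tick accumulates delta seconds into an internal timer.
; A looping timer started on BeginPlay compares that value to LifeTime every tenth of a second and destroys the actor when it is reached.
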(event `self.ReceiveBeginPlay`
  ; Begin
  (`KismetSystemLibrary.K2_SetTimerDelegate` (delegate `Chek_Lifetime`) 0.1 true))

(event `Chek_Lifetime`
  (if (>= (`self.Internal_Timer`) (`self.LifeTime`))
    (`self.K2_DestroyActor`)))

(event `self.ReceiveTick`
  (params (DeltaSeconds :type "Float (single-precision)"))
  ; Event tick
  (set `self.Internal_Timer` (+ DeltaSeconds (`self.Internal_Timer`))))

(fn `UserConstructionScript`)
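; VR sniper rifle with grab components for main grip, bolt lever and secondary handle.
; Main grip toggles per-hand input mappings; that hand's trigger calls TryToShoot, whose line-trace impulse is blocked by a hardcoded false condition.
; While held, a looping timer projects the hand onto the rifle axis to slide the clamped lever.
; Lever thresholds drive chambering with casing ejection and a ready-to-shoot flag, though the latter's branch is unreachable.
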(event `self.ReceiveBeginPlay`
  (bind _sniper (`self.Sniper`))
  (bind _relativelocation_x (`KismetMathLibrary.BreakVector` (`SceneComponent.RelativeLocation` (`self.Sniper_lever_V4`))))
  ; Begin
  (`self.EnableInput` (`GameplayStatics.GetPlayerController` 0))
  (`SceneComponent.K2_AttachToComponent` (`self.Lunette de rendu`) _sniper "None" "KeepRelative" "KeepRelative" "KeepRelative" true)
  (`SceneComponent.K2_AttachToComponent` (`self.SceneCaptureComponent2D`) _sniper "None" "KeepRelative" "KeepRelative" "KeepRelative" true)
  (`SceneComponent.K2_AttachToComponent` (`self.Magazine`) _sniper "None" "KeepRelative" "KeepRelative" "KeepRelative" true)
  (`SceneComponent.K2_AttachToComponent` (`self.BulletPosEject`) null "None" "KeepRelative" "KeepRelative" "KeepRelative" true)
  (bind _asvrpawn (cast `/Game/VRTemplate/Blueprints/VRPawn` (`GameplayStatics.GetPlayerPawn` 0)))
  (bind _output_get (set `self.VRPawn ref` _asvrpawn))
  (add `/Game/VRTemplate/Blueprints/VRPawn.Shoot Left` _output_get (`|CreateDelegate` :!event `Shoot_Left_internal`))
  (add `/Game/VRTemplate/Blueprints/VRPawn.Shoot Right` _output_get (`|CreateDelegate` :!event `Shoot_Right_internal`))
  (bind _output_get_2 (set `self.LeverStartPosX` _relativelocation_x))
  (set `self.LeverPosNeedToShoot` (+ _output_get_2 -10.0))
  (bind _output_get_3 (set `self.LeverMaxX` (+ _relativelocation_x -52.0)))
  (set `self.LeverPosNeedToReload` (+ _output_get_3 20.0)))

(event `self.GrabComponent_Main.OnGrabbed`
  (bind _grabcomponent_main (`self.GrabComponent_Main`))
  (bind _returnvalue (`|EnumEquality` (`/Game/VRTemplate/Blueprints/GrabComponent.GetHeldByHand` _grabcomponent_main) "Right"))
  ; Grab
  (`self.EnableInput` (`GameplayStatics.GetPlayerController` 0))
  (message `/Game/VRTemplate/Blueprints/BPI_PawnAnim.HideUnhideHand` (`ActorComponent.GetOwner` (`/Game/VRTemplate/Blueprints/GrabComponent.MotionControllerRef` _grabcomponent_main)) false _returnvalue)
  (`EnhancedInputSubsystemInterface.AddMappingContext` (pcsubsystem `EnhancedInputLocalPlayerSubsystem` (`GameplayStatics.GetPlayerController` 0)) (select `bool` _returnvalue :`false` "/Game/VRTemplate/Input/IMC_Weapon_Left.IMC_Weapon_Left" :`true` "/Game/VRTemplate/Input/IMC_Weapon_Right.IMC_Weapon_Right" :!type "InputMappingContext Object Reference") 1 (struct))
  (set `self.MainIsGrab?` true))

(event `self.GrabComponent_Main.OnDropped`
  (bind _grabcomponent_main (`self.GrabComponent_Main`))
  (bind _returnvalue (`|EnumEquality` (`/Game/VRTemplate/Blueprints/GrabComponent.GetHeldByHand` _grabcomponent_main) "Right"))
  ; Grab
  (`self.DisableInput` (`GameplayStatics.GetPlayerController` 0))
  (message `/Game/VRTemplate/Blueprints/BPI_PawnAnim.HideUnhideHand` (`ActorComponent.GetOwner` (`/Game/VRTemplate/Blueprints/GrabComponent.MotionControllerRef` _grabcomponent_main)) false _returnvalue)
  (`EnhancedInputSubsystemInterface.RemoveMappingContext` (pcsubsystem `EnhancedInputLocalPlayerSubsystem` (`GameplayStatics.GetPlayerController` 0)) (select `bool` _returnvalue :`false` "/Game/VRTemplate/Input/IMC_Weapon_Left.IMC_Weapon_Left" :`true` "/Game/VRTemplate/Input/IMC_Weapon_Right.IMC_Weapon_Right" :!type "InputMappingContext Object Reference") (struct))
  (set `self.MainIsGrab?` false))

(event `Shoot_Left_internal`
  ; Shoot
  (if (`|EnumEquality` (`/Game/VRTemplate/Blueprints/GrabComponent.GetHeldByHand` (`self.GrabComponent_Main`)) "Left")
    (`self.TryToShoot` :!label _label)))

(event `Shoot_Right_internal`
  ; Shoot
  (if (`|EnumEquality` (`/Game/VRTemplate/Blueprints/GrabComponent.GetHeldByHand` (`self.GrabComponent_Main`)) "Right")
    (goto _label)))

(event `TryToShoot`
  (bind _nozzle (`self.Nozzle`))
  (bind _returnvalue (`SceneComponent.K2_GetComponentLocation` _nozzle))
  (bind _returnvalue_2 (+ _returnvalue (* (`SceneComponent.GetForwardVector` _nozzle) 500.0)))
  ; Try To Shoot
  (if (and (`self.MainIsGrab?`) (`self.Bullet_in_chamber`) (`self.ReadyToShoot`) false)
    (bind _outhit (`KismetSystemLibrary.LineTraceSingle` :`Start` _returnvalue :`End` _returnvalue_2 :`TraceChannel` "TraceTypeQuery1" :`DrawDebugType` "ForDuration"))
    (set `self.Bullet_in_chamber` false)
    (`PrimitiveComponent.AddImpulse` (`.HitComponent` (`GameplayStatics.BreakHitResult` _outhit)) _returnvalue_2 "None" true)
    (else
      (`KismetSystemLibrary.PrintString` "Unauthorised shooting"))))

(event `UpdateLever`
  (bind _sniper (`self.Sniper`))
  (bind _bulletposeject (`self.BulletPosEject`))
  (bind _sniper_lever_v4 (`self.Sniper_lever_V4`))
  (bind (_relativelocation_x _relativelocation_y _relativelocation_z) (`KismetMathLibrary.BreakVector` (`SceneComponent.RelativeLocation` _sniper_lever_v4)))
  (bind _returnvalue_x (`KismetMathLibrary.BreakVector` (`KismetMathLibrary.InverseTransformLocation` (`SceneComponent.K2_GetComponentToWorld` (`self.Sniper`)) (`KismetMathLibrary.FindClosestPointOnLine` (`self.HandTamponLocation`) (`SceneComponent.K2_GetComponentLocation` _sniper) (`SceneComponent.GetForwardVector` _sniper)))))
  (bind _returnvalue (`KismetMathLibrary.FClamp` _returnvalue_x (`self.LeverMaxX`) (`self.LeverStartPosX`)))
  ; Lever
  (if (and (`/Game/VRTemplate/Blueprints/GrabComponent.bIsHeld` (`self.GrabComponent_Lever`)) (`self.MainIsGrab?`))
    (if (`self.RightHand`)
      (set `self.HandTamponLocation` (`SceneComponent.K2_GetComponentLocation` (`/Game/VRTemplate/Blueprints/VRPawn.MotionControllerRightGrip` (`self.VRPawn ref`))))
      (else
        (set `self.HandTamponLocation` (`SceneComponent.K2_GetComponentLocation` (`/Game/VRTemplate/Blueprints/VRPawn.MotionControllerLeftGrip` (`self.VRPawn ref`))))))
    (`SceneComponent.K2_SetRelativeLocation` _sniper_lever_v4 (`KismetMathLibrary.MakeVector` _returnvalue _relativelocation_y _relativelocation_z) false false)
    (if (>= _returnvalue (`self.LeverPosNeedToReload`))
      (if (not (`self.Bullet_in_chamber`))
        (set `self.Bullet_in_chamber` true)
        (bind _returnvalue_2 (`|SpawnActorFromClass` "/Game/__Game/Blueprints/Sniper/Bp_Empty_Bullet.Bp_Empty_Bullet_C" (`SceneComponent.K2_GetComponentToWorld` _bulletposeject) "Undefined" "MultiplyWithRoot" null null))
        (`PrimitiveComponent.AddForce` (`/Game/__Game/Blueprints/Sniper/Bp_Empty_Bullet.bullet` _returnvalue_2) (* (`SceneComponent.GetRightVector` _bulletposeject) 300.0) "None" false)
        (`KismetSystemLibrary.PrintString` "Reload complete"))
      (elif (>= _returnvalue (`self.LeverPosNeedToShoot`))
        (if (not (`self.ReadyToShoot`))
          (set `self.ReadyToShoot` true)
          (`KismetSystemLibrary.PrintString` "Ready To Shoot"))))))

(event `self.GrabComponent_Lever.OnGrabbed`
  ; Grab component Lever
  (`KismetSystemLibrary.DelayUntilNextTick`)
  (set `self.RightHand` (== (`/Game/VRTemplate/Blueprints/VRPawn.HeldComponentRight` (`self.VRPawn ref`)) (`self.GrabComponent_Lever`)))
  (bind _returnvalue (`KismetSystemLibrary.K2_SetTimerDelegate` (`|CreateDelegate` :!event `UpdateLever`) 0.1 true true))
  (set `self.Timer` _returnvalue))

(event `self.GrabComponent_Lever.OnDropped`
  ; Stop lever Update
  (`KismetSystemLibrary.K2_ClearAndInvalidateTimerHandle` (`self.Timer`)))

(event `self.GrabComponent_Poignée.OnGrabbed`
  ; Secondary Grab
  (set `self.SecondaryIsGrab?` true))

(event `self.GrabComponent_Poignée.OnDropped`
  ; Secondary Grab
  (set `self.SecondaryIsGrab?` false))

(fn `UserConstructionScript`)